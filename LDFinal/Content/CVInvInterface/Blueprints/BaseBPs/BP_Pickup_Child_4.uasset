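; Child pickup Blueprint for an inventory system, holding only item-specific settings while the parent supplies the shared behavior.
; OnExamine copies the item's variables, placeholder examine text and inventory info struct into inherited fields, then calls the parent.
; The construction script sets the mesh's custom depth stencil so takable and non-takable items highlight green or orange on hover.
; Tick continuously rotates the pickup mesh around its local pitch axis.
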(event EventTick
  (params (DeltaSeconds :type Float%20%28single-precision%29))
  ;[1 0 0.2892] Set custom variables unique to this item within the OnExamine function. Note this Blueprint contains only information that is unique to it. All the other functionality is stored in the Parent.
  (Transformation|AddLocalRotation (Variables|Default|GetPickupMesh) (* (Math|Rotator|MakeRotator 0.0 2e+01 0.0) DeltaSeconds) false false))

(fn ConstructionScript
  (if (Utilities|Enum|Equal(Enum) (Variables|Default|GetThisTakableOrNot) "NewEnumerator0")
    ;[1 1 1] If Takable, set Stencil Value to 252 - Highlight Green when hovered over
    (Rendering|SetCustomDepthStencilValue (Variables|Default|GetPickupMesh) 252)
    (else
      ;[1 1 1] If NOT Takable, set Stencil Value to 254 - Highlight Orange when hovered over
      (Rendering|SetCustomDepthStencilValue (Variables|Default|GetPickupMesh) 254)))
  (|CallParentFunction))

(fn OnExamine
  (params (Character :type First%20Person%20Character%20Object%20Reference))
  (bind _thisinvdropactorclass (Variables|Default|GetThisInvDropActorClass))
  (bind _thisinventoryclass (Variables|Default|GetThisInventoryClass))
  (Variables|Default|SetItemDescription "Relace this text. This text appears on the Examine screen when first clicking on a Pickup item. 
 
Use SHIFT-RETURN to do a line/paragraph break. 
 
This text is unique to the examine screen. You can have the same or different information in the description area after you take the item into your inventory.")
  (Variables|Default|SetInventoryClass _thisinventoryclass)
  (Variables|Default|SetClassOfBP _thisinvdropactorclass)
  (Variables|Default|SetItemInfo (Utilities|Struct|MakeBS_InvInfoStruct (Variables|Default|GetThisItemName) "" _thisinvdropactorclass 0 (Variables|Default|GetThisInvIconImage) 0 _thisinventoryclass (Variables|Default|GetThisIsUsable)))
  (Variables|Default|SetTakableOrNot (Variables|Default|GetThisTakableOrNot))
  (bind _success (|CallParentFunction 0))
  (return _success))