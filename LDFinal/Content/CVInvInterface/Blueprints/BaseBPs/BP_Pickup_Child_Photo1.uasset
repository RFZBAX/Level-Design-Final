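; Child pickup Blueprint for an examinable photo with a personal memory about a Chinese teaching group, leaving shared functionality to its parent.
; OnExamine fills the description, inventory classes, item info struct and takable state before calling the parent.
; The construction script picks the mesh's custom depth stencil value from takable state, and Tick spins the mesh in pitch.
; Initphoto1 creates a dynamic material instance from the photo material.
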(event EventTick
  (params (DeltaSeconds :type Float%20%28single-precision%29))
  ;[1 0 0.2892] Set custom variables unique to this item within the OnExamine function. Note this Blueprint contains only information that is unique to it. All the other functionality is stored in the Parent.
  (Transformation|AddLocalRotation (Variables|Default|GetPickupMesh) (* (Math|Rotator|MakeRotator 0.0 2e+01 0.0) DeltaSeconds) false false))

(fn ConstructionScript
  (bind _pickupmesh (Variables|Default|GetPickupMesh))
  (if (Utilities|Enum|Equal(Enum) (Variables|Default|GetThisTakableOrNot) "NewEnumerator0")
    (Rendering|SetCustomDepthStencilValue _pickupmesh 252)
    (else
      (Rendering|SetCustomDepthStencilValue _pickupmesh 254)))
  (|CallParentFunction))

(fn OnExamine
  (params (Character :type First%20Person%20Character%20Object%20Reference))
  (bind _thisinvdropactorclass (Variables|Default|GetThisInvDropActorClass))
  (bind _thisinventoryclass (Variables|Default|GetThisInventoryClass))
  (Variables|Default|SetItemDescription "I have so many great memories related to the Chinese teaching group. True self, The Stranger Around... We've talked and wrote about so many unforgetable topics. Not to mention the poetry festival, the play festival, etc.. I always love the Chinese teaching group.")
  (Variables|Default|SetInventoryClass _thisinventoryclass)
  (Variables|Default|SetClassOfBP _thisinvdropactorclass)
  (Variables|Default|SetItemInfo (Utilities|Struct|MakeBS_InvInfoStruct (Variables|Default|GetThisItemName) "" _thisinvdropactorclass 0 (Variables|Default|GetThisInvIconImage) 0 _thisinventoryclass (Variables|Default|GetThisIsUsable)))
  (Variables|Default|SetTakableOrNot (Variables|Default|GetThisTakableOrNot))
  (bind _success (|CallParentFunction 0))
  (return _success))

(fn Initphoto1
  (bind _returnvalue (Rendering|Material|CreateDynamicMaterialInstance (Variables|Default|GetPickupMesh) 0 "/Game/Models/Photo/Photo_txt_1.Photo_txt_1" "None" :!class /Script/Engine.PrimitiveComponent))
  (return _returnvalue))