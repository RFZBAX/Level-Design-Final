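; Interactable tree that turns into a board actor when the axe check passes on interaction.
; An empty HUD inventory shows a timed dialog; otherwise it loops over all BP_InventoryActor instances in the level, comparing ItemID to AxeID.
; A match spawns BoardActor and destroys the tree, while each mismatch runs the dialog branch.
; The axe check reads level actors rather than inventory contents, and the graph's locked-drawer comment does not match this logic.
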(event EventOnInteract
  (params (Character :type First%20Person%20Character%20Object%20Reference))
  ;[1 1 1] Locked Drawer - check to see if you have the KEY in your INVENTORY - if NOT say that its locked. If YES unlock and set Drawer is unlocked Var for next time. so player can get rid of Key.
  (if (< (Utilities|Array|Length (Variables|/Game/CVInvInterface/Blueprints/Widgets/BPW_INVExamine.BPW_INVExamine_C|GetInventoryUE (Variables|/Game/CVInvInterface/Blueprints/FirstPersonCharacter.FirstPersonCharacter_C|GetGameHUDWidgetUE Character))) 1)
    ;[1 1 1] UMG Dialog Box for locked drawer
    (bind _returnvalue (UserInterface|CreateWidget "/Game/CVInvInterface/Blueprints/Widgets/BPW_DialogBox.BPW_DialogBox_C" :!label _label))
    (Class|BPIDialogTxtMessage|DialogTxtMessage(Message) _returnvalue (Variables|Default|GetText))
    (if (Variables|Default|GetAlreadyViewable)
      (Viewport|RemoveAllWidgets)
      (else
        (UserInterface|Viewport|AddtoViewport _returnvalue 0)
        (Variables|Default|SetAlreadyViewable true)
        (Utilities|FlowControl|Delay 3.0)
        (Widget|RemovefromParent _returnvalue)))
    (Variables|Default|SetAlreadyViewable false)
    (else
      (bind _outactors (Actor|GetAllActorsOfClass "/Game/CVInvInterface/Blueprints/InventoryActorBPS/BP_InventoryActor.BP_InventoryActor_C"))
      (for _array_element _outactors
        (if (== (Variables|/Game/CVInvInterface/Blueprints/InventoryActorBPS/BP_InventoryActor.BP_InventoryActor_C|GetItemID _array_element) (Variables|Default|GetAxe%20ID))
          (Game|SpawnActorfromClass "/Game/BoardActor.BoardActor_C" (Variables|Default|Getboard) "Undefined" 0 0)
          (Actor|DestroyActor)
          (else
            (goto _label)))))))

(fn ConstructionScript
  (|CallParentFunction))